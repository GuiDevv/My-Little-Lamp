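; Player camera that turns mouse gestures into interactions with the BP_LittleLamp character.
; Tick traces under the cursor and sends focus/defocus messages, pausing while a press on a "Focuble" component is active.
; Release dispatches by component tag: head drags rotate or impulse it, vertical leg drags impulse that leg, and quick leg clicks or IA_TAP stop the head.
; Holding on the head shines the lamp, raising happiness and resetting sparks.
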(event `self.ReceiveBeginPlay`
  (set `PlayerController.bShowMouseCursor` true (`GameplayStatics.GetPlayerController` 0))
  (bind _returnvalue (`GameplayStatics.GetActorOfClass` "/Game/MyLittleLamp/Core/BP_LittleLamp.BP_LittleLamp_C"))
  (set `self.LittleLamp` _returnvalue))

(event `self.ReceiveTick`
  (params (DeltaSeconds :type "Float (single-precision)"))
  (bind (_bblockinghit _binitialoverlap _time _distance _location _impactpoint _normal _impactnormal _physmat _hitactor _hitcomponent) (`GameplayStatics.BreakHitResult` (`PlayerController.GetHitResultUnderCursorByChannel` (`GameplayStatics.GetPlayerController` 0) "TraceTypeQuery1" true)))
  (if (`self.PlayerInput`)
    (if (`self.ActionTrigged`)
      _
      (elif (!= (`self.Hit Component`) _hitcomponent)
        (bind _hit_component (`self.Hit Component`)
          (:`then`
            (message `/Game/MyLittleLamp/Core/BP_InteractInterface.OnDefocus` (`self.HitActor`) _hit_component))
          (:`else`
            _))
        (message `/Game/MyLittleLamp/Core/BP_InteractInterface.On Focus` _hitactor _hitcomponent)
        (set `self.Hit Component` _hitcomponent)
        (set `self.HitActor` _hitactor)))))

(event `EnhancedInput|/Game/MyLittleLamp/Inputs/IA_MLL`
  (params (ActionValue :type Boolean) (ElapsedSeconds :type "Float (double-precision)") (TriggeredSeconds :type "Float (double-precision)") (InputAction :type "InputAction Object Reference" :default "/Game/MyLittleLamp/Inputs/IA_MLL.IA_MLL"))
  (bind (_locationx _locationy) (`WidgetLayoutLibrary.GetMousePositionScaledByDPI` (`GameplayStatics.GetPlayerController` 0)))
  (bind _returnvalue (== (`.HitComponent` (`GameplayStatics.BreakHitResult` (`PlayerController.GetHitResultUnderCursorByChannel` (`GameplayStatics.GetPlayerController` 0) "TraceTypeQuery1" true))) (`self.Hit Component`)))
  (:`Triggered`
    (if (> TriggeredSeconds 1.0)
      (if (`ActorComponent.ComponentHasTag` (`self.Hit Component`) "Head")
        (`/Game/MyLittleLamp/Core/BP_LittleLamp.Shine Lamp` (`self.LittleLamp`) _returnvalue)
        (if _returnvalue
          (`|ExecutionSequence`
            (:`then_0`
              (`/Game/MyLittleLamp/Core/StatusComponent.Modify Happy` (`/Game/MyLittleLamp/Core/BP_LittleLamp.StatusComponent` (`self.LittleLamp`)) 0.005))
            (:`then_1`
              (`KismetSystemLibrary.Delay` 0.15)
              (`NiagaraComponent.ResetSystem` (`/Game/MyLittleLamp/Core/BP_LittleLamp.Sparks` (`self.LittleLamp`)))))))))
  (:`Started`
    (bind _hit_component (`self.Hit Component`)
      (:`then`
        (if (`ActorComponent.ComponentHasTag` _hit_component "Focuble")
          (set `self.PressedLocation` (`KismetMathLibrary.MakeVector2D` _locationx _locationy))
          (set `self.ActionTrigged` true)))
      (:`else`)))
  (:`Completed`
    (if (`self.ActionTrigged`)
      (bind _hit_component_2 (`self.Hit Component`)
        (:`then`
          (set `self.ActionTrigged` false)
          (`/Game/MyLittleLamp/Core/BP_LittleLamp.Shine Lamp` (`self.LittleLamp`) false)
          (switch `name` (`|GetArrayItem` (`ActorComponent.ComponentTags` _hit_component_2))
            (:`Head`
              (`self.HeadInteraction` TriggeredSeconds))
            (:`Right_Leg`
              (`self.Leg Interaction` TriggeredSeconds))
            (:`Left_Leg`
              (`self.Leg Interaction` TriggeredSeconds true))))
        (:`else`)))))

(event `EnhancedInput|/Game/MyLittleLamp/Inputs/IA_TAP`
  (params (ActionValue :type Boolean) (ElapsedSeconds :type "Float (double-precision)") (TriggeredSeconds :type "Float (double-precision)") (InputAction :type "InputAction Object Reference" :default "/Game/MyLittleLamp/Inputs/IA_TAP.IA_TAP"))
  (:`Completed`
    (`/Game/MyLittleLamp/Core/BP_LittleLamp.Stop Head` (`self.LittleLamp`))))

(fn `HeadInteraction`
  (params (TriggedTime :type "Float (double-precision)"))
  (bind (_pressedlocation_x _pressedlocation_y) (`KismetMathLibrary.BreakVector2D` (`self.PressedLocation`)))
  (bind (_releasedlocation_x _releasedlocation_y) (`KismetMathLibrary.BreakVector2D` (`self.ReleasedLocation`)))
  (bind _pressedlocation_x_2 (`KismetMathLibrary.BreakVector2D` (`self.PressedLocation`)))
  (bind _releasedlocation_x_2 (`KismetMathLibrary.BreakVector2D` (`self.ReleasedLocation`)))
  (bind _pressedlocation_x_3 (`KismetMathLibrary.BreakVector2D` (`self.PressedLocation`)))
  (bind _releasedlocation_x_3 (`KismetMathLibrary.BreakVector2D` (`self.ReleasedLocation`)))
  (bind (_locationx _locationy) (`WidgetLayoutLibrary.GetMousePositionScaledByDPI` (`GameplayStatics.GetPlayerController` 0)))
  (bind _returnvalue (`KismetMathLibrary.Distance2D` (`self.PressedLocation`) (`self.ReleasedLocation`)))
  (bind _returnvalue_2 (- _pressedlocation_y _releasedlocation_y))
  (bind _returnvalue_3 (`KismetMathLibrary.Abs` _returnvalue_2))
  (bind _returnvalue_4 (`KismetMathLibrary.MapRangeClamped` _returnvalue_3 0.0 500.0 0.0 1.0))
  (set `self.ReleasedLocation` (`KismetMathLibrary.MakeVector2D` _locationx _locationy))
  (if (not (> _returnvalue_3 150.0))
    (if (> (`KismetMathLibrary.Abs` (- _pressedlocation_x_2 _releasedlocation_x_3)) 150.0)
      ;[1 1 1] Drag
      (`/Game/MyLittleLamp/Core/BP_LittleLamp.Rotate Head` (`self.LittleLamp`) (* (`KismetMathLibrary.MapRangeClamped` _returnvalue 0.0 1000.0 0.0 15.0) (`KismetMathLibrary.SelectFloat` 1.0 -1.0 (< _releasedlocation_x_2 _pressedlocation_x_3))) (`KismetMathLibrary.MapRangeClamped` _returnvalue 0.0 1000.0 0.0 2.0)))
    (else
      ;[1 1 1] Impulse
      (`/Game/MyLittleLamp/Core/BP_LittleLamp.Impulse Head` (`self.LittleLamp`) (`KismetMathLibrary.SelectFloat` (* _returnvalue_4 -1.0) _returnvalue_4 (< _returnvalue_2 0.0))))))

(fn `Leg Interaction`
  (params (TriggedTime :type "Float (double-precision)") (Left_Leg :type Boolean))
  (bind (_pressedlocation_x _pressedlocation_y) (`KismetMathLibrary.BreakVector2D` (`self.PressedLocation`)))
  (bind (_releasedlocation_x _releasedlocation_y) (`KismetMathLibrary.BreakVector2D` (`self.ReleasedLocation`)))
  (bind (_locationx _locationy) (`WidgetLayoutLibrary.GetMousePositionScaledByDPI` (`GameplayStatics.GetPlayerController` 0)))
  (bind _returnvalue (- _pressedlocation_y _releasedlocation_y))
  (bind _returnvalue_2 (`KismetMathLibrary.Abs` _returnvalue))
  (bind _returnvalue_3 (`KismetMathLibrary.MapRangeClamped` _returnvalue_2 0.0 500.0 0.0 1.0))
  (if (> TriggedTime 0.1)
    (set `self.ReleasedLocation` (`KismetMathLibrary.MakeVector2D` _locationx _locationy))
    (if (not (not (> _returnvalue_2 100.0)))
      ;[1 1 1] Impulse
      (`/Game/MyLittleLamp/Core/BP_LittleLamp.ImpulseLeg` (`self.LittleLamp`) (`KismetMathLibrary.SelectFloat` _returnvalue_3 (* _returnvalue_3 -1.0) (< _returnvalue 0.0)) (`local.Left_Leg`)))
    (else
      (`/Game/MyLittleLamp/Core/BP_LittleLamp.Stop Head` (`self.LittleLamp`)))))

(fn `UserConstructionScript`)