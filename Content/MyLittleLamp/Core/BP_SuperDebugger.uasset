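; BP_SuperDebugger is a debug actor that toggles level lighting visibility shortly after play begins.
; BeginPlay caches all spot lights plus the first directional light, sky light and post-process volume, then calls DisableLights after a short delay and prints a message.
; DisableLights inverts each spot light's visibility and sets directional and sky light visibility from the negated directional light state.
; The post-process reference is stored but unused.
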(event `self.ReceiveBeginPlay`
  (`|ExecutionSequence`
    (:`then_0`
      (bind _outactors (`GameplayStatics.GetAllActorsOfClass` "/Script/Engine.SpotLight"))
      (set `self.SpotLights` _outactors)
      (bind _returnvalue (`GameplayStatics.GetActorOfClass` "/Script/Engine.DirectionalLight"))
      (set `self.Directional Light` _returnvalue)
      (bind _returnvalue_2 (`GameplayStatics.GetActorOfClass` "/Script/Engine.PostProcessVolume"))
      (set `self.Post Process` _returnvalue_2)
      (bind _returnvalue_3 (`GameplayStatics.GetActorOfClass` "/Script/Engine.SkyLight"))
      (set `self.Sky Ligth` _returnvalue_3))
    (:`then_1`
      (`KismetSystemLibrary.Delay` 2.0)
      (`self.DisableLights`)
      (`KismetSystemLibrary.PrintString` "Hello"))))

(fn `DisableLights`
  (bind _lightcomponent (`Light.LightComponent` (`self.Directional Light`)))
  (for _array_element (`self.SpotLights`)
    (bind _spotlightcomponent (`SpotLight.SpotLightComponent` _array_element))
    (`SceneComponent.SetVisibility` _spotlightcomponent (not (`SceneComponent.IsVisible` _spotlightcomponent)) false))
  (`SceneComponent.SetVisibility` _lightcomponent (not (`SceneComponent.IsVisible` _lightcomponent)) false)
  (`SceneComponent.SetVisibility` (`Actor.RootComponent` (`self.Sky Ligth`)) (not (`SceneComponent.IsVisible` _lightcomponent)) false))

(fn `UserConstructionScript`)