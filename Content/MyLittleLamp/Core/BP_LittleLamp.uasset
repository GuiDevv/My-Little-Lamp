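; Interactive lamp character actor with a spinnable head, physics-reactive head and legs, focus outlines and a dimmable light.
; Rotating again mid-spin triggers a timer-driven boost with a spark ring, and further input during boost plays a head-spin Level Sequence.
; Impulses to head or legs raise sadness or anger on StatusComponent.
; Looping timers ramp light intensity, emissive and spark count together, while helper functions recolor, resize and replay Niagara effects.
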(event `self.ReceiveBeginPlay`
  (bind _outactor (`LevelSequencePlayer.CreateLevelSequencePlayer` (`self.SpinHeadAnimation`)))
  (bind _output_get (set `self.SHActor` _outactor))
  (`MovieSceneSequencePlayer.SetPlayRate` (`LevelSequenceActor.SequencePlayer` _output_get) 2.0))

(event `Boost Event`
  (params (Duration :type "Float (double-precision)"))
  (bind _sparkring (`self.SparkRing`))
  (set `self.IsBoosting` true)
  (if (`TimelineComponent.IsPlaying` (`self.RotateHeadTimeline`))
    (`TimelineComponent.Stop` (`self.RotateHeadTimeline`))
    (`KismetSystemLibrary.K2_SetTimerDelegate` (delegate `BoostAction`) 0.05 true))
  (`|ExecutionSequence`
    (:`then_0`
      (`NiagaraComponent.SetVariableLinearColor` _sparkring "VortexColor" (* (`LightComponentBase.GetLightColor` (`self.PointLight`)) (struct :`R` 15.0 :`G` 15.0 :`B` 15.0 :`A` 1.0)))
      (`NiagaraComponent.SetVariableFloat` _sparkring "SpawnRate" (`KismetMathLibrary.MapRangeClamped` (`KismetMathLibrary.Abs` (`self.RotateStrenght`)) 0.0 15.0 1000.0 5000.0))
      (`NiagaraComponent.ResetSystem` _sparkring))
    (:`then_1`
      (`KismetSystemLibrary.RetriggerableDelay` Duration)
      (`KismetSystemLibrary.K2_ClearTimer` null "BoostAction")
      (set `self.IsBoosting` false)
      (`TimelineComponent.Play` (`self.RotateHeadTimeline`)))))

(event `BoostAction`
  (`SceneComponent.K2_AddLocalRotation` (`self.HeadCape`) (`KismetMathLibrary.MakeRotator` 0.0 0.0 (* 0.9 (`KismetMathLibrary.SelectFloat` -15.0 15.0 (< (`self.RotateStrenght`) 0.0)))) false false))

(event `Rotate Head`
  (params (RotateStrenght :type "Float (double-precision)") (RotateDuration :type "Float (double-precision)"))
  (bind _rotateheadtimeline (`self.RotateHeadTimeline`))
  (bind _isboosting (`self.IsBoosting`))
  (bind _sequenceplayer (`LevelSequenceActor.SequencePlayer` (`self.SHActor`)))
  (if (`TimelineComponent.IsPlaying` (`self.RotateHeadTimeline`))
    (if _isboosting
      _
      (elif (== (+ (`KismetMathLibrary.Abs` (`self.RotateStrenght`)) (`KismetMathLibrary.Abs` RotateStrenght)) (`KismetMathLibrary.Abs` (+ (`self.RotateStrenght`) RotateStrenght)))
        (`self.Boost Event` 1.5)))
    (elif _isboosting
      (if (`MovieSceneSequencePlayer.IsPlaying` (`LevelSequenceActor.SequencePlayer` (`self.SHActor`)))
        _
        (elif (< (`self.RotateStrenght`) 0.0)
          (`MovieSceneSequencePlayer.PlayReverse` _sequenceplayer)
          (else
            (`MovieSceneSequencePlayer.Play` _sequenceplayer))))
      (else
        (set `self.RotateStrenght` RotateStrenght)
        (`TimelineComponent.SetPlayRate` _rotateheadtimeline (/ 1.0 RotateDuration))
        (`TimelineComponent.PlayFromStart` _rotateheadtimeline)))))

(event `/Game/MyLittleLamp/Core/BP_InteractInterface.On Focus`
  (params (Mesh :type "PrimitiveComponent Object Reference"))
  (if (`ActorComponent.ComponentHasTag` Mesh "Focuble")
    (`PrimitiveComponent.SetCustomDepthStencilValue` Mesh 2)
    (`PrimitiveComponent.SetRenderCustomDepth` Mesh true)
    (if (`ActorComponent.ComponentHasTag` Mesh "Head")
      (`PrimitiveComponent.SetRenderCustomDepth` (`self.Head`) true))))

(event `/Game/MyLittleLamp/Core/BP_InteractInterface.OnDefocus`
  (params (Mesh :type "PrimitiveComponent Object Reference"))
  (if (`ActorComponent.ComponentHasTag` Mesh "Focuble")
    (`PrimitiveComponent.SetRenderCustomDepth` Mesh false)
    (if (`ActorComponent.ComponentHasTag` Mesh "Head")
      (`PrimitiveComponent.SetRenderCustomDepth` (`self.Head`) false))))

(event `Impulse Head`
  (params (Strenght :type "Float (double-precision)"))
  (bind _arrow (`self.Arrow`))
  (bind _returnvalue (`SceneComponent.K2_GetComponentLocation` _arrow))
  (`PrimitiveComponent.AddImpulse` (`self.Head`) (- _returnvalue (+ (* (`SceneComponent.GetForwardVector` _arrow) (* 5000.0 Strenght)) _returnvalue)) "None" true)
  (if (not (`/Game/MyLittleLamp/Core/StatusComponent.IgnoreInteraction` (`self.StatusComponent`)))
    (`/Game/MyLittleLamp/Core/StatusComponent.Modify Sad` (`self.StatusComponent`) 0.1)))

(event `Stop Head`
  (`PrimitiveComponent.SetAllPhysicsLinearVelocity` (`self.Head`) (0.0 0.0 0.0) false))

(event `Shine Lamp`
  (params (Increase :type Boolean))
  (bind _isshinning (`self.IsShinning`))
  (if Increase
    (if (not _isshinning)
      (set `self.IsShinning` true)
      (`KismetSystemLibrary.K2_ClearTimer` null "Decrease Lamp Intensity")
      (`KismetSystemLibrary.K2_SetTimerDelegate` (`|CreateDelegate` :!event `Raise Lamp Intensity`) 0.05 true))
    (elif _isshinning
      (set `self.IsShinning` false)
      (`KismetSystemLibrary.K2_ClearTimer` null "Raise Lamp Intensity")
      (`KismetSystemLibrary.K2_SetTimerDelegate` (`|CreateDelegate` :!event `Decrease Lamp Intensity`) 0.05 true))))

(event `ImpulseLeg`
  (params (Strenght :type "Float (double-precision)") (Left_Leg :type Boolean))
  (bind _returnvalue (select `bool` Left_Leg :`false` (`self.Arrow2`) :`true` (`self.Arrow1`)))
  (bind _returnvalue_2 (`SceneComponent.K2_GetComponentLocation` _returnvalue))
  (`PrimitiveComponent.AddImpulse` (select `bool` Left_Leg :`false` (`self.Right_Leg`) :`true` (`self.Left_Leg`)) (- _returnvalue_2 (+ _returnvalue_2 (* (`SceneComponent.GetForwardVector` _returnvalue) (* 5000.0 Strenght)))) "None" true)
  (if (not (`/Game/MyLittleLamp/Core/StatusComponent.IgnoreInteraction` (`self.StatusComponent`)))
    (`/Game/MyLittleLamp/Core/StatusComponent.Modify Angry` (`self.StatusComponent`) 0.1)))

(fn `Decrease Lamp Intensity`
  (bind _pointlight (`self.PointLight`))
  (bind _returnvalue (`KismetMathLibrary.FClamp` (- (`LightComponentBase.Intensity` _pointlight) (/ (`self.IntensityDelta`) 2.0)) 1000.0 10000.0))
  (`LightComponent.SetIntensity` _pointlight _returnvalue)
  (`MeshComponent.SetScalarParameterValueOnMaterials` (`self.Head`) "Emissive" (/ _returnvalue 10000.0))
  (`NiagaraComponent.SetNiagaraVariableInt` (`self.Sparks`) "SpawnCount" (`KismetMathLibrary.Round` (`KismetMathLibrary.MapRangeClamped` _returnvalue 1000.0 10000.0 10.0 50.0)))
  (if (== _returnvalue 1000.0)
    (`KismetSystemLibrary.K2_ClearTimer` null "Decrease Lamp Intensity")))

(fn `ParticleColorEditor`
  (params (Particle :type "/Game/MyLittleLamp/Core/EParticles Enum" :default "NewEnumerator0") (BaseColor :type "LinearColor Structure") (SecondaryColor :type "LinearColor Structure"))
  (bind _returnvalue (* BaseColor (struct :`R` 15.0 :`G` 15.0 :`B` 15.0 :`A` 1.0)))
  (switch `/Game/MyLittleLamp/Core/EParticles` Particle
    (:`NewEnumerator0`
      (bind _spawned_particle (`self.Spawned Particle` :!label _label)
        (:`then`
          (`NiagaraComponent.SetVariableLinearColor` _spawned_particle "SparkColorBase" _returnvalue)
          (`NiagaraComponent.SetVariableLinearColor` _spawned_particle "SparkColorSecondary" (* SecondaryColor (struct :`R` 15.0 :`G` 15.0 :`B` 15.0 :`A` 1.0))))
        (:`else`)))
    (:`NewEnumerator1`
      (`NiagaraComponent.SetVariableLinearColor` (`self.Sparks`) "SparkColor" _returnvalue :!label _label_2))
    (:`NewEnumerator2`
      (`NiagaraComponent.SetVariableLinearColor` (`self.SparkRing`) "VortexColor" _returnvalue :!label _label_3))
    (:`NewEnumerator3`
      (`|ExecutionSequence`
        (:`then_0`
          (goto _label))
        (:`then_1`
          (goto _label_2))
        (:`then_2`
          (goto _label_3))))))

(fn `ParticlePlay`
  (params (Particle :type "/Game/MyLittleLamp/Core/EParticles Enum" :default "NewEnumerator0"))
  (switch `/Game/MyLittleLamp/Core/EParticles` Particle
    (:`NewEnumerator0`
      (bind _returnvalue (`NiagaraFunctionLibrary.SpawnSystemAtLocation` (select `/Game/MyLittleLamp/Core/EParticles` Particle :`NewEnumerator0` "/Game/MyLittleLamp/VFX_Project/NS_SparkExplosion.NS_SparkExplosion" :!type "NiagaraSystem Object Reference") (`SceneComponent.K2_GetComponentLocation` (`self.Explosion`)) :!label _label))
      (set `self.Spawned Particle` _returnvalue))
    (:`NewEnumerator1`
      (`NiagaraComponent.ResetSystem` (`self.Sparks`) :!label _label_2))
    (:`NewEnumerator2`
      (`NiagaraComponent.ResetSystem` (`self.SparkRing`) :!label _label_3))
    (:`NewEnumerator3`
      (`|ExecutionSequence`
        (:`then_0`
          (goto _label))
        (:`then_1`
          (goto _label_2))
        (:`then_2`
          (goto _label_3))))))

(fn `ParticleSpawnEditor`
  (params (Particle :type "/Game/MyLittleLamp/Core/EParticles Enum" :default "NewEnumerator0") (Count :type Integer))
  (switch `/Game/MyLittleLamp/Core/EParticles` Particle
    (:`NewEnumerator0`
      (bind _spawned_particle (`self.Spawned Particle` :!label _label)
        (:`then`
          (`NiagaraComponent.SetVariableInt` _spawned_particle "Spawn Count" Count))
        (:`else`)))
    (:`NewEnumerator1`
      (`NiagaraComponent.SetNiagaraVariableInt` (`self.Sparks`) "SpawnCount" Count :!label _label_2))
    (:`NewEnumerator3`
      (`|ExecutionSequence`
        (:`then_0`
          (goto _label))
        (:`then_1`
          (goto _label_2))))))

(fn `Raise Lamp Intensity`
  (bind _pointlight (`self.PointLight`))
  (bind _returnvalue (`KismetMathLibrary.FClamp` (+ (`LightComponentBase.Intensity` _pointlight) (`self.IntensityDelta`)) 1000.0 10000.0))
  (`LightComponent.SetIntensity` _pointlight _returnvalue)
  (`MeshComponent.SetScalarParameterValueOnMaterials` (`self.Head`) "Emissive" (/ _returnvalue 10000.0))
  (`NiagaraComponent.SetNiagaraVariableInt` (`self.Sparks`) "SpawnCount" (`KismetMathLibrary.Round` (`KismetMathLibrary.MapRangeClamped` _returnvalue 1000.0 10000.0 10.0 50.0)))
  (if (== _returnvalue 10000.0)
    (`KismetSystemLibrary.K2_ClearTimer` null "Raise Lamp Intensity")
    (`LightComponent.SetIntensity` (`self.PointLight`) 10000.0)))

(fn `UserConstructionScript`)